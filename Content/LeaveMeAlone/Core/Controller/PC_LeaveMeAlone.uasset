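; PC_LeaveMeAlone is the player controller Blueprint, which opens the pause menu on the Pause input.
; If not already paused, it sets OnPause, stops weapon fire through the character's LMAWeaponComponent and pauses the game.
; It then creates and shows WBP_Pause, switches to UI-only input focused on that widget and shows the mouse cursor.
; Nothing in this graph clears OnPause or resumes the game.
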(event `InputAction|Pause`
  (params (Key :type "Key Structure"))
  (:`Pressed`
    (if (not (`self.OnPause`))
      (set `self.OnPause` true)
      (`LMAWeaponComponent.StopFire` (`self.GetComponentByClass` (`GameplayStatics.GetPlayerCharacter` 0) "/Script/LeaveMeAlone.LMAWeaponComponent"))
      (`GameplayStatics.SetGamePaused` true)
      (bind _returnvalue (`|CreateWidget` "/Game/LeaveMeAlone/Widgets/HUD/WBP_Pause.WBP_Pause_C"))
      (bind _output_get (set `self.Pause Widget` _returnvalue))
      (`UserWidget.AddToViewport` _output_get 0)
      (`WidgetBlueprintLibrary.SetInputMode_UIOnlyEx` self _output_get)
      (set `self.bShowMouseCursor` true))))

(fn `UserConstructionScript`)